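; BP_Start is a startup pawn that bootstraps the player into the game's main spaceship.
; On BeginPlay it spawns BP_MainSpaceShip at its own transform, then casts its controller to BP_RTFController.
; The controller unpossesses it, is initialized with the ship and possesses the ship's main character.
; A W_TestWidget receives the ship reference and is added to the viewport.
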(event EventBeginPlay
  (bind _returnvalue (Game|SpawnActorfromClass "/Game/Resources/MainSpaceShip/Blueprints/Logic/BP_MainSpaceShip.BP_MainSpaceShip_C" (Transformation|GetActorTransform) "Undefined" "MultiplyWithRoot" 0 0))
  (bind _asbp_rtfcontroller (Utilities|Casting|CastToBP_RTFController (Pawn|GetController)))
  (Pawn|UnPossess _asbp_rtfcontroller)
  (Class|RTFController|InitControllerInfo _asbp_rtfcontroller _returnvalue)
  (Pawn|Possess _asbp_rtfcontroller (Class|MainSpaceShip|GetMainCharacter _returnvalue))
  (bind _returnvalue_2 (UserInterface|CreateWidget "/Game/UI/W_TestWidget.W_TestWidget_C"))
  (Variables|/Game/UI/W_TestWidget.W_TestWidget_C|SetSpaceShipRef _returnvalue_2 _returnvalue)
  (UserInterface|Viewport|AddtoViewport _returnvalue_2 0))

(event Collision|EventActorBeginOverlap
  (params (OtherActor :type Actor%20Object%20Reference)))

(event EventTick
  (params (DeltaSeconds :type Float%20%28single-precision%29)))

(fn ConstructionScript)